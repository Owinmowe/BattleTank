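; Mortar_BP is a mortar weapon built from body, dome and barrel meshes that aims and fires through a TankAiming component.
; On BeginPlay it assigns the three static meshes and gives each the Tank_green material.
; It then initializes TankAiming with the barrel, the dome as turret and Projectile_BP as the projectile class.
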(event `self.ReceiveBeginPlay`
  (bind _mortar_body (`self.Mortar Body`))
  (bind _mortar_dome (`self.Mortar Dome`))
  (bind _mortar_barrel (`self.Mortar Barrel`))
  (`StaticMeshComponent.SetStaticMesh` _mortar_body "/Game/Mortar_Model/mortar_body.mortar_body")
  (`PrimitiveComponent.SetMaterial` _mortar_body 0 "/Game/Tank_Model/tank_green.tank_green")
  (`StaticMeshComponent.SetStaticMesh` _mortar_dome "/Game/Mortar_Model/mortar_dome.mortar_dome")
  (`PrimitiveComponent.SetMaterial` _mortar_dome 0 "/Game/Tank_Model/tank_green.tank_green")
  (`StaticMeshComponent.SetStaticMesh` _mortar_barrel "/Game/Mortar_Model/mortar_barrel.mortar_barrel")
  (`PrimitiveComponent.SetMaterial` _mortar_barrel 0 "/Game/Tank_Model/tank_green.tank_green")
  (`TankAimingComponent.Initialize` (`self.TankAiming`) (`self.Mortar Barrel`) (`self.Mortar Dome`) "/Game/Tank_Model/Projectile_BP.Projectile_BP_C"))

(fn `UserConstructionScript`)